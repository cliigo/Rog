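; BP_RogCharacter is a character Blueprint that manages its initial Gameplay Ability System ability sets.
; When the ASC initializes, it grants InitAbilitySet to the RogAbilitySystemComponent and stores the returned handles.
; On EndPlay it passes those handles back to remove the granted sets.
; A Collect component's overlap event only prints the overlapping actor's name.
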(event `self.Collect.OnComponentBeginOverlap`
  (params (OverlappedComponent :type "PrimitiveComponent Object Reference") (OtherActor :type "Actor Object Reference") (OtherComp :type "PrimitiveComponent Object Reference") (OtherBodyIndex :type Integer) (bFromSweep :type Boolean) (SweepResult :type "HitResult Structure (by ref)"))
  (`KismetSystemLibrary.PrintString` (`KismetSystemLibrary.GetDisplayName` OtherActor)))

(event `self.K2_OnASCInit`
  ;[1 1 1] InitAbilitySet
  (bind _asrog_ability_system_component (cast `RogAbilitySystemComponent` (`AbilitySystemBlueprintLibrary.GetAbilitySystemComponent` self)))
  (bind _outgrantedhandles (`RogAbilityFunctionLibrary.AddAbilitySetToASC` _asrog_ability_system_component (`self.InitAbilitySet`) null))
  (set `self.Out Granted Handles` _outgrantedhandles))

(event `self.ReceiveEndPlay`
  (params (EndPlayReason :type "EEndPlayReason Enum" :default "Destroyed"))
  ;[1 1 1] 移除技能集合
  (bind _asrog_ability_system_component (cast `RogAbilitySystemComponent` (`AbilitySystemBlueprintLibrary.GetAbilitySystemComponent` null)))
  (`RogAbilityFunctionLibrary.TakeFormAbilitySystem` _asrog_ability_system_component (`self.Out Granted Handles`)))

(fn `UserConstructionScript`)