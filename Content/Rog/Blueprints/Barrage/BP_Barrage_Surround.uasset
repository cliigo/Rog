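; BP_Barrage_Surround is a barrage actor that circles around a reference actor (MaterActor).
; Each Tick advances a timer that wraps at AllTime, then converts its fraction of the period into an angle for Sin and Cos.
; The resulting vector, with HeightOffset as Z, is scaled by Dis and added to MaterActor's location, so height also scales with radius.
; The position is set directly, without sweep.
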(event `self.ReceiveTick`
  (params (DeltaSeconds :type "Float (single-precision)"))
  (bind _alltime (`self.AllTime`))
  ;[1 1 1] 更新时间，计算当前时间百分比
  (bind _output_get (set `self.UpdateTime` (mod (+ DeltaSeconds (`self.UpdateTime`)) _alltime)))
  (bind _returnvalue (* (/ _output_get _alltime) (`KismetMathLibrary.MultiplyByPi` 2.0)))
  (`self.K2_SetActorLocation` (+ (* (`KismetMathLibrary.MakeVector` (`KismetMathLibrary.Sin` _returnvalue) (`KismetMathLibrary.Cos` _returnvalue) (`self.HeightOffset`)) (`self.Dis`)) (`self.K2_GetActorLocation` (`|ConvertAsset` (`self.MaterActor`))))))

(fn `UserConstructionScript`
  (`parent.UserConstructionScript`))