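; BP_AttackerFlySword is an unfinished attacker Blueprint meant to manage a pool of flying swords in slots.
; BeginPlay requests five slots through UpdateSlot, which on a count change deactivates existing swords' root components and calls CreateNewSword with the difference.
; CreateNewSword's loop is empty, with its list-add and deactivate nodes disconnected, so no swords are created.
; UpdateSwordPos is an empty stub, and Tick and overlap events are disabled.
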(event `self.ReceiveBeginPlay`
  (`self.Update Slot` 5))

(fn `CreateNewSword`
  (params (CreateCount :type Integer))
  (if (> CreateCount 0)
    (for _ (range (+ CreateCount 1))
      _)))

(fn `HildeAllOldSword`
  (bind _slotlist (`self.SlotList`))
  ;[1 1 1] 隐藏旧的actor
  (for _index (range (+ (`KismetArrayLibrary.Array_Length` _slotlist) 1))
    (`ActorComponent.SetActive` (`Actor.RootComponent` (`|GetArrayItem` _slotlist _index)) false false)))

(fn `Update Slot`
  (params (SlotCount :type Integer))
  (bind _slotcount (`self.SlotCount`))
  (if (not (== SlotCount _slotcount))
    (`|ExecutionSequence`
      (:`then_0`
        (`self.HildeAllOldSword`)
        (`self.CreateNewSword` (- SlotCount _slotcount)))
      (:`then_1`
        (set `self.SlotCount` SlotCount)))))

(fn `UpdateSwordPos`)

(fn `UserConstructionScript`)